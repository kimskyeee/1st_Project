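; BP_Enemy is an enemy actor that tracks health and ragdolls when killed.
; On any damage it subtracts the amount from EnemyHP and prints the remaining value while above zero.
; At zero or below, it turns on physics simulation and query-and-physics collision on its Mesh.
; BeginPlay, overlap, Tick and the construction script are empty.
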(event EventBeginPlay)

(event Collision|EventActorBeginOverlap
  (params (OtherActor :type Actor%20Object%20Reference)))

(event EventTick
  (params (DeltaSeconds :type Float%20%28single-precision%29)))

(event Game|Damage|EventAnyDamage
  (params (Damage :type Float%20%28single-precision%29) (DamageType :type Damage%20Type%20Object%20Reference) (InstigatedBy :type Controller%20Object%20Reference) (DamageCauser :type Actor%20Object%20Reference))
  (bind _mesh (Variables|Character|GetMesh))
  ;[0.15 0.15 0.15 0.5] Enemy HP
  (Variables|Default|SetEnemyHP (- (Variables|Default|GetEnemyHP) Damage))
  (if (> (Variables|Default|GetEnemyHP) 0.0)
    (Development|PrintText (Utilities|Text|ToText(Float) (Variables|Default|GetEnemyHP) "HalfToEven"))
    (else
      (Physics|SetSimulatePhysics _mesh true)
      (Collision|SetCollisionEnabled _mesh "QueryAndPhysics"))))

(fn ConstructionScript)