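; BP_Bullet is a projectile Actor for the player's weapon that moves itself every frame.
; BeginPlay caches the BP_PlayerCharcter found in the level.
; Each Tick runs that character's current SpringArm forward vector through the bullet's own transform, scales it by Speed and delta time, and applies it as a swept location offset.
; The direction is re-read every frame, and no hit handling is present.
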(event EventTick
  (params (DeltaSeconds :type Float%20%28single-precision%29))
  ;[0.15 0.15 0.15 0.5] 이동하고싶다
  ;;[0.15 0.15 0.15 0.5] P
  (Transformation|SetActorLocation (+ (* DeltaSeconds (* (Math|Transform|TransformDirection (Transformation|GetActorTransform) (Math|Vector|GetForwardVector (Variables|/Game/CustomContents/Player/BP_PlayerCharcter.BP_PlayerCharcter_C|GetSpringArm (stale EventBeginPlay _returnvalue)))) (Variables|Default|GetSpeed))) (Transformation|GetActorLocation)) true false))

(event EventBeginPlay
  (bind _returnvalue (Actor|GetActorOfClass "/Game/CustomContents/Player/BP_PlayerCharcter.BP_PlayerCharcter_C")))

(fn ConstructionScript)