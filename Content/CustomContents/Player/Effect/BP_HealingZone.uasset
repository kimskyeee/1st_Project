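; BP_HealingZone is an actor that heals the player over time while an overlap is active.
; Begin overlap starts a looping timer that calls HealPlayer every second and destroys the zone after a short delay; end overlap clears the timer.
; Neither overlap event filters the other actor, and HealPlayer always increases health on player character 0 through its BPCStatSystem component.
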(event Collision|EventActorBeginOverlap
  (params (OtherActor :type Actor%20Object%20Reference))
  (bind _returnvalue (Utilities|Time|SetTimerbyFunctionName 0 "HealPlayer" 1.0 true))
  (Variables|Default|SetNewVar _returnvalue)
  (Utilities|FlowControl|Delay 6.0)
  (Actor|DestroyActor))

(event Collision|EventActorEndOverlap
  (params (OtherActor :type Actor%20Object%20Reference))
  (Utilities|Time|ClearandInvalidateTimerbyHandle (Variables|Default|GetNewVar)))

(fn ConstructionScript)

(fn HealPlayer
  (bind _asbp_player_charcter (Utilities|Casting|CastToBP_PlayerCharcter (Game|GetPlayerCharacter 0)))
  (Default|IncreaseHealth (Variables|/Game/CustomContents/Player/BP_PlayerCharcter.BP_PlayerCharcter_C|GetBPC_StatSystem _asbp_player_charcter) 4e+01))