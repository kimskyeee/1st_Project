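; Behavior tree task that makes an AI pawn chase the actor stored in a blackboard key.
; Each tick it moves the pawn straight toward the target at blackboard Speed scaled by delta time, without pathfinding or sweep.
; The world-space direction is applied as a local offset, so pawn rotation affects the movement.
; Once within blackboard TargetRange it finishes as failed, and it never reports success.
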(event EventReceiveTickAI
  (params (OwnerController :type AI%20Controller%20Object%20Reference) (ControlledPawn :type Pawn%20Object%20Reference) (DeltaSeconds :type Float%20%28single-precision%29))
  (bind _returnvalue (AI|GetBlackboard OwnerController))
  (bind _asactor (Utilities|Casting|CastToActor (AI|Components|Blackboard|GetValueasObject _returnvalue (Variables|Default|GetTargetObj))))
  (bind _asactor_2 (Utilities|Casting|CastToActor ControlledPawn))
  (if (<= (Transformation|GetDistanceTo _asactor _asactor_2) (Class|BlackboardComponent|GetValueasFloat _returnvalue (Variables|Default|GetTargetRange)))
    (AI|BehaviorTree|FinishExecute false)
    (else
      (CallFunction|Moveto _asactor_2 _asactor (* DeltaSeconds (Class|BlackboardComponent|GetValueasFloat _returnvalue (Variables|Default|GetSpeed)))))))

(fn Moveto
  (params (Actor :type Actor%20Object%20Reference) (OtherActor :type Actor%20Object%20Reference) (SpeedPerTick :type Float%20%28double-precision%29))
  (Transformation|AddActorLocalOffset Actor (* (Math|Vector|Normalize (- (Transformation|GetActorLocation OtherActor) (Transformation|GetActorLocation Actor)) 1.0) SpeedPerTick) false false)
  (return))