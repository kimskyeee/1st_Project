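; Behavior tree decorator that passes when the AI's controlled pawn is within a threshold distance of its target.
; The condition check compares the pawn's distance to the target against NearestValue, inclusive.
; GetTarget reads the TargetObj key from the controller's blackboard and casts it to Actor.
; A failed cast yields no actor, which the distance check uses without a validity test.
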(fn PerformConditionCheckAI
  (params (OwnerController :type AI%20Controller%20Object%20Reference) (ControlledPawn :type Pawn%20Object%20Reference))
  (return (<= (Transformation|GetDistanceTo ControlledPawn (AI|GetTarget OwnerController)) (Variables|Default|GetNearestValue))))

(fn GetTarget
  (params (AIController :type AI%20Controller%20Object%20Reference))
  (bind _asactor (Utilities|Casting|CastToActor (AI|Components|Blackboard|GetValueasObject (AI|GetBlackboard AIController) (Variables|Default|GetTargetObj)))
    (:then
      (return _asactor))
    (:CastFailed
      (return 0))))