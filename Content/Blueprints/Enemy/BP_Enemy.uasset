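; BP_Enemy is an enemy Blueprint that shoots bullets from two alternating fire points.
; ShootGun spawns a BP_EnemyBullet at the FireLeft or FireRight component transform, flipping IsLeftHand after each shot to switch sides.
; Nothing in this file calls ShootGun, and the construction script is empty.
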(fn ConstructionScript)

(fn ShootGun
  (if (Variables|Default|GetIsLeftHand)
    (Game|SpawnActorfromClass "/Game/Blueprints/Enemy/BP_EnemyBullet.BP_EnemyBullet_C" (Transformation|GetWorldTransform (Variables|Default|GetFireLeft)) "Undefined" "MultiplyWithRoot" 0 0)
    (else
      (Game|SpawnActorfromClass "/Game/Blueprints/Enemy/BP_EnemyBullet.BP_EnemyBullet_C" (Transformation|GetWorldTransform (Variables|Default|GetFireRight)) "Undefined" "MultiplyWithRoot" 0 0)))
  (Variables|Default|SetIsLeftHand (not (Variables|Default|GetIsLeftHand)))
  (return))