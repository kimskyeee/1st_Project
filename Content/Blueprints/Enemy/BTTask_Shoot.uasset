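; Behavior tree task that makes the controlled BP_Enemy fire its gun in a burst.
; The AI tick event casts the pawn, then loops through a short Delay and ShootGun, counting shots in ShootCount.
; When the count matches MaxShootCount, it resets to 1 and the task finishes as failed rather than succeeded.
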(event EventReceiveExecuteAI
  (params (OwnerController :type AI%20Controller%20Object%20Reference) (ControlledPawn :type Pawn%20Object%20Reference)))

(event EventReceiveTickAI
  (params (OwnerController :type AI%20Controller%20Object%20Reference) (ControlledPawn :type Pawn%20Object%20Reference) (DeltaSeconds :type Float%20%28single-precision%29))
  (bind _asbp_enemy (Utilities|Casting|CastToBP_Enemy ControlledPawn))
  (Utilities|FlowControl|Delay 0.27 :!label _label)
  (Default|ShootGun _asbp_enemy)
  (if (== (Variables|Default|GetMaxShootCount) (Variables|Default|GetShootCount))
    (Variables|Default|SetShootCount 1)
    (AI|BehaviorTree|FinishExecute false)
    (else
      (Variables|Default|SetShootCount (+ (Variables|Default|GetShootCount) 1))
      (goto _label))))