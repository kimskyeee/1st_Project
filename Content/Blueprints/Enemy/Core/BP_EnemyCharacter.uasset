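; BP_EnemyCharacter is the core enemy character, delegating health and skills to its CombatComponent.
; Incoming damage goes to that component, whose death event destroys the actor after a brief delay.
; CastDefaultSkill activates the skill table's default attack with the actor's owner, leaving its target input unused.
; A LineTrace helper runs a Camera-channel trace and returns the hit and result.
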(event Custom|OnDied_Event
  (Utilities|FlowControl|Delay 0.2)
  (Actor|DestroyActor))

(event Game|Damage|EventAnyDamage
  (params (Damage :type Float%20%28single-precision%29) (DamageType :type Damage%20Type%20Object%20Reference) (InstigatedBy :type Controller%20Object%20Reference) (DamageCauser :type Actor%20Object%20Reference))
  (Default|DamageHealth (Variables|Default|GetCombatComponent) Damage))

(event EventBeginPlay
  (EventDispatchers|BindEventtoOnDied (Variables|Default|GetCombatComponent) (delegate Custom|OnDied_Event)))

(fn ConstructionScript)

(fn CastDefaultSkill
  (params (Cast%20Target :type Actor%20Object%20Reference))
  (Default|Activate (.defaultattack (Variables|/Game/Blueprints/Enemy/Core/Component/CombatComponent.CombatComponent_C|GetSkillTable (Variables|Default|GetCombatComponent))) (Components|GetOwner))
  (return))

(fn LineTrace
  (params (Start :type Vector) (End :type Vector))
  (bind (_outhit _returnvalue) (Collision|LineTraceByChannel Start End "TraceTypeQuery2" false 0 "None"))
  (return _outhit _returnvalue))