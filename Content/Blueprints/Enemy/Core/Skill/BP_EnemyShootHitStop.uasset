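; Enemy shooting skill that fires an instant line-trace attack when activated on an enemy character.
; It spends one ammo from the CombatComponent, then traces from the FireSocket along its forward vector out to Range.
; The trace uses LineTraceComponent on the caster's own capsule, so it tests only that component rather than the world.
; The hit actor receives damage equal to the CombatComponent's Attack, with no hit check or hit-stop logic.
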(fn Activate
  (params (Actor :type Actor%20Object%20Reference))
  (|CallParentFunction Actor)
  (bind _asbp_enemy_character (Utilities|Casting|CastToBP_EnemyCharacter Actor))
  (CallFunction|AttackLineTrace _asbp_enemy_character)
  (return))

(fn CalculateShootLocation
  (params (TargetLocation :type Vector) (ForwardVector :type Vector))
  (return (+ TargetLocation (* ForwardVector (Variables|Default|GetRange)))))

(fn AttackLineTrace
  (params (Caster :type Actor%20Object%20Reference))
  (bind _asbp_enemy_character (Utilities|Casting|CastToBP_EnemyCharacter Caster))
  (Default|UseAmmo (Variables|/Game/Blueprints/Enemy/Core/BP_EnemyCharacter.BP_EnemyCharacter_C|GetCombatComponent _asbp_enemy_character) 1)
  (bind _outhit (Collision|LineTraceComponent (Variables|/Script/Engine.Character|GetCapsuleComponent _asbp_enemy_character) (Transformation|GetWorldLocation (Variables|/Game/Blueprints/Enemy/Core/BP_EnemyCharacter.BP_EnemyCharacter_C|GetFire%20Socket _asbp_enemy_character)) (CallFunction|CalculateShootLocation (Transformation|GetWorldLocation (Variables|/Game/Blueprints/Enemy/Core/BP_EnemyCharacter.BP_EnemyCharacter_C|GetFire%20Socket _asbp_enemy_character)) (Math|Vector|GetForwardVector (Variables|/Game/Blueprints/Enemy/Core/BP_EnemyCharacter.BP_EnemyCharacter_C|GetFire%20Socket _asbp_enemy_character))) true true false))
  (Game|Damage|ApplyDamage (.hitactor _outhit) (Math|Conversions|ToFloat(Integer) (Variables|/Game/Blueprints/Enemy/Core/Component/CombatComponent.CombatComponent_C|GetAttack (Variables|/Game/Blueprints/Enemy/Core/BP_EnemyCharacter.BP_EnemyCharacter_C|GetCombatComponent _asbp_enemy_character))) 0 0)
  (return))