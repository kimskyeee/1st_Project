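; Game state Blueprint that runs a timed match, declaring defeat when time runs out and presenting the game-over sequence.
; On game start, timers drive a per-second remaining-time countdown and the loss at expiry, which fires the game-over event.
; Game over spawns a widget and plays a timeline that drives its fade and global time dilation, shows Korean victory or defeat text, then opens the main menu.
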(event Custom|GameStartEvent_Event
  (CallFunction|GameStart)
  (Utilities|Time|SetTimerbyEvent (delegate Custom|GameDefeatEvent_Event) (Math|Conversions|ToFloat(Integer) (Variables|PlayTime|GetRemainTime)) false true)
  (Utilities|Time|SetTimerbyFunctionName 0 "TimerMove" 1.0 true))

(event Custom|GameOverEvent_Event
  (bind _returnvalue (UserInterface|CreateWidget "/Game/Blueprints/Widget/WBP_GameOverWidget.WBP_GameOverWidget_C" (Game|GetPlayerController 0)))
  (UserInterface|Viewport|AddtoViewport _returnvalue 0)
  (bind (_direction _timelinevalue _slow) (Timeline|Finish Play)
    (:Update
      (Variables|/Script/UMG.Widget|SetRenderOpacity (Variables|/Game/Blueprints/Widget/WBP_GameOverWidget.WBP_GameOverWidget_C|GetBorderUI _returnvalue) _timelinevalue)
      (Utilities|Time|SetGlobalTimeDilation _slow)
      (if (Utilities|Enum|Equal(Enum) (Variables|GameState|GetGameOver) "NewEnumerator1")
        ;[0.15 0.15 0.15 0.5] TODO: 추후 SetText가 아닌 UI 기반의 함수 호출로 변경
        (Rendering|Components|TextRender|SetText (Variables|/Game/Blueprints/Widget/WBP_GameOverWidget.WBP_GameOverWidget_C|GetGameOverDisplayText _returnvalue) "승리")
        (else
          (Rendering|Components|TextRender|SetText (Variables|/Game/Blueprints/Widget/WBP_GameOverWidget.WBP_GameOverWidget_C|GetGameOverDisplayText _returnvalue) "패배"))))
    (:Finished
      (Game|OpenLevel(byObjectReference) "/Game/Blueprints/Level/MainMenu.MainMenu"))))

(event Custom|GameDefeatEvent_Event
  (CallFunction|SetGameLoss)
  (Default|CallGameOverEvent))

(event EventBeginPlay
  (EventDispatchers|BindEventtoGameStartEvent (delegate Custom|GameStartEvent_Event))
  (EventDispatchers|BindEventtoGameOverEvent (delegate Custom|GameOverEvent_Event))
  (Variables|PlayTime|SetCurrentRemainTime (Variables|PlayTime|GetRemainTime))
  (EventDispatchers|BindEventtoGameDefeatEvent (delegate Custom|GameDefeatEvent_Event)))

(fn ConstructionScript)

(fn GameStart
  (bind _remaintime (Variables|PlayTime|GetRemainTime))
  (Variables|PlayTime|SetCurrentRemainTime _remaintime)
  (Utilities|Time|SetTimerbyFunctionName 0 "SetGameLoss" (Math|Conversions|ToFloat(Integer) _remaintime))
  (return))

(fn GameOverTodo
  (if (not (== (Variables|GameState|GetGameOver) 0))
    (if (not (Variables|GameState|GetIsAlreadyOver))
      (Variables|GameState|SetIsAlreadyOver true))))

(fn SetGameLoss
  (Variables|GameState|SetGameOver "NewEnumerator2")
  (CallFunction|GameOverTodo)
  (return))

(fn TimerMove
  (if (not (== (Variables|PlayTime|GetCurrentRemainTime) 0.0))
    (Variables|PlayTime|SetCurrentRemainTime (- (Variables|PlayTime|GetCurrentRemainTime) 1.0))
    (return)))

(fn ShowGameOverView)