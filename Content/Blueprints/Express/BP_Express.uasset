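; Escort payload actor that, after a HUD countdown opens the door and starts the game, floats up and travels along checkpoints built from offsets.
; Each Tick, a sphere trace gates movement: it advances only with the player nearby and no living enemy detected.
; When blocked it stops, then after a delay retreats toward the previous checkpoint.
; Progress and remaining distance feed the HUD; the final checkpoint triggers GameOver on the game state.
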(event EventTick
  (params (DeltaSeconds :type Float%20%28single-precision%29))
  (bind _result (CallFunction|CanMove))
  (CallFunction|CheckNearestEntity)
  (switch Utilities|FlowControl|Switch|SwitchonE_ExpressStatus (Variables|Movement|GetStatus)
    (:NewEnumerator0
      (if _result
        (CallFunction|MovetoGoal DeltaSeconds (CallFunction|GetMovetoLocation DeltaSeconds))
        (if (CallFunction|IsMoreThanCheckPoint (CallFunction|GetBetweenNextCheckPointDistance) (CallFunction|GetBetweenCurrentPosandNextCheckPoint))
          (if (>= (Variables|DirectionPoint|GetCurrentDirectPoint) (- (Utilities|Array|Length (Variables|DirectionPoint|GetMoveToDirectionList)) 1))
            (Actor|Tick|SetActorTickEnabled false)
            (bind _asbp_game_play_state (Utilities|Casting|CastToBP_GamePlayState (Game|GetGameState)))
            (Variables|/Game/Blueprints/GameMode/BP_GamePlayState.BP_GamePlayState_C|SetGameOver _asbp_game_play_state "NewEnumerator1")
            (Default|CallGameOverEvent _asbp_game_play_state)
            (else
              (Variables|DirectionPoint|SetCurrentDirectPoint (+ (Variables|DirectionPoint|GetCurrentDirectPoint) 1)))))
        (else
          (Variables|Movement|SetStatus "NewEnumerator6"))))
    (:NewEnumerator2
      (CallFunction|FloattoStart DeltaSeconds))
    (:NewEnumerator3
      (if _result
        (Variables|Movement|SetStatus "NewEnumerator0")
        (else
          (CallFunction|MovetoBack DeltaSeconds))))
    (:NewEnumerator5
      (if _result
        (Variables|Movement|SetStatus "NewEnumerator0")))
    (:NewEnumerator6
      (Variables|Movement|SetStatus "NewEnumerator5")
      (Utilities|Time|SetTimerbyFunctionName 0 "SetGoBack" (Variables|Default|GetDelayTime)))))

(event EventBeginPlay
  (bind _returnvalue (Transformation|GetActorLocation))
  (for _array_element (Variables|DirectionPoint|GetDirectionList)
    (Utilities|Array|Add (Variables|DirectionPoint|GetMoveToDirectionList) (+ _returnvalue _array_element))
    (Variables|DirectionPoint|SetStartPinPoint _returnvalue)
    (bind _asbp_playercontroller (Utilities|Casting|CastToBP_Playercontroller (Pawn|GetController (Game|Player|GetPlayerPawn 0))))
    (bind _returnvalue_2 (UserInterface|CreateWidget "/Game/Blueprints/Widget/WBP_GameHUD.WBP_GameHUD_C" _asbp_playercontroller))
    (bind _output_get (Variables|Default|SetHUD _returnvalue_2))
    (UserInterface|Viewport|AddtoViewport _output_get 0)
    (Variables|Game/Pause|SetRemainPauseTimeMs (Variables|Game/Pause|GetPauseTimeMs))
    (bind _returnvalue_3 (Utilities|Time|SetTimerbyFunctionName 0 "MovePauseTimer" 0.1 true))
    (Variables|Game/Pause|SetPauseTimerHandle _returnvalue_3)))

(fn ConstructionScript)

(fn IsMoreThanCheckPoint
  (params (BetweenCheckPointDistance :type Float%20%28double-precision%29) (BetweenCurrentPosAndCheckPoint :type Float%20%28double-precision%29))
  (return (<= (Class|KismetMathLibrary|AbsInt64 (- (Class|KismetMathLibrary|FCeil64 BetweenCheckPointDistance) (Class|KismetMathLibrary|FCeil64 BetweenCurrentPosAndCheckPoint))) 3)))

(fn GetBetweenNextCheckPointDistance
  (if (== (Variables|DirectionPoint|GetCurrentDirectPoint) 0)
    (return (Math|Vector|Distance(Vector) (Utilities|Array|Get(acopy) (Variables|DirectionPoint|GetMoveToDirectionList) (Variables|DirectionPoint|GetCurrentDirectPoint)) (Variables|DirectionPoint|GetStartPinPoint)))
    (else
      (return (Math|Vector|Distance(Vector) (Utilities|Array|Get(acopy) (Variables|DirectionPoint|GetMoveToDirectionList) (Variables|DirectionPoint|GetCurrentDirectPoint)) (Utilities|Array|Get(acopy) (Variables|DirectionPoint|GetMoveToDirectionList) (- (Variables|DirectionPoint|GetCurrentDirectPoint) 1)))))))

(fn GetBetweenCurrentPosandNextCheckPoint
  (if (== (Variables|DirectionPoint|GetCurrentDirectPoint) 0)
    (return (+ (Math|Vector|Distance(Vector) (Utilities|Array|Get(acopy) (Variables|DirectionPoint|GetMoveToDirectionList) (Variables|DirectionPoint|GetCurrentDirectPoint)) (Variables|DirectionPoint|GetStartPinPoint)) (Math|Vector|Distance(Vector) (Utilities|Array|Get(acopy) (Variables|DirectionPoint|GetMoveToDirectionList) (Variables|DirectionPoint|GetCurrentDirectPoint)) (Transformation|GetActorLocation))))
    (else
      (return (+ (Math|Vector|Distance(Vector) (Utilities|Array|Get(acopy) (Variables|DirectionPoint|GetMoveToDirectionList) (Variables|DirectionPoint|GetCurrentDirectPoint)) (Utilities|Array|Get(acopy) (Variables|DirectionPoint|GetMoveToDirectionList) (- (Variables|DirectionPoint|GetCurrentDirectPoint) 1))) (Math|Vector|Distance(Vector) (Utilities|Array|Get(acopy) (Variables|DirectionPoint|GetMoveToDirectionList) (Variables|DirectionPoint|GetCurrentDirectPoint)) (Transformation|GetActorLocation)))))))

(fn MovetoGoal
  (params (DeltaSecond :type Float%20%28double-precision%29) (MoveToLocation :type Vector))
  (bind _result (CallFunction|GetCurrentDistancetoMove))
  (bind _result_2 (CallFunction|GetTotalExpressDistance))
  (bind _hud (Variables|Default|GetHUD))
  (Transformation|SetActorLocation (+ MoveToLocation (Transformation|GetActorLocation)) false false)
  (Transformation|SetActorRotation (Math|Interpolation|RInterpTo (Transformation|GetActorRotation) (Math|Rotator|MakeRotfromX MoveToLocation) DeltaSecond 2.0))
  (Variables|Default|SetPrevPercent (Math|Float|Max(Float) (Variables|Default|GetPrevPercent) (/ _result _result_2)))
  (Progress|SetPercent (Variables|/Game/Blueprints/Widget/WBP_GameHUD.WBP_GameHUD_C|GetCurrentBar _hud) (Math|Float|Max(Float) (Variables|Default|GetPrevPercent) (/ _result _result_2)))
  (Default|SetRemainDistance _hud (- _result_2 _result))
  (return))

(fn CheckNearestEntity
  (bind _returnvalue (Transformation|GetActorLocation))
  (Variables|Condition|SetIsNearPlayerTemp false)
  (Variables|Condition|SetIsNearEnemyTemp false)
  (bind _outhits (Collision|MultiSphereTraceByChannel _returnvalue _returnvalue (Variables|Movement|GetCheckRadius) "TraceTypeQuery2" false 0 "ForOneFrame"))
  (for _array_element _outhits
    (Utilities|Casting|CastToBP_PlayerCharcter (.hitactor _array_element)
      (:then
        (Variables|Condition|SetIsNearPlayerTemp true))
      (:CastFailed
        _))
    (bind _asbp_enemy_character (Utilities|Casting|CastToBP_EnemyCharacter (.hitactor _array_element)))
    (Variables|Condition|SetIsNearEnemyTemp (not (Variables|/Game/Blueprints/Enemy/Core/Component/CombatComponent.CombatComponent_C|GetIsDied (Variables|/Game/Blueprints/Enemy/Core/BP_EnemyCharacter.BP_EnemyCharacter_C|GetCombatComponent _asbp_enemy_character)))))
  (Variables|Condition|SetIsNearPlayer (Variables|Condition|GetIsNearPlayerTemp))
  (Variables|Condition|SetIsNearEnemy (Variables|Condition|GetIsNearEnemyTemp))
  (return))

(fn FloattoStart
  (params (DeltaTime :type Float%20%28double-precision%29%20%28by%20ref%29))
  (bind _express (Variables|Default|GetExpress))
  (Transformation|AddLocalOffset _express (Math|Vector|MakeVector 0.0 0.0 (* (* DeltaTime (Variables|Movement/Float|GetFloatHeight)) (Variables|Movement/Float|GetFloatSpeed))) false false)
  (Default|SetRemainDistance (Variables|Default|GetHUD) (CallFunction|GetTotalExpressDistance))
  (if (> (.z (Variables|/Script/Engine.SceneComponent|GetRelativeLocation _express)) (Variables|Movement/Float|GetFloatHeight))
    (Variables|Movement|SetStatus "NewEnumerator0")
    (else
      (return))))

(fn GetMovetoLocation
  (params (DeltaSecond :type Float%20%28double-precision%29%20%28by%20ref%29))
  (return (* (Math|Vector|Normalize (- (Utilities|Array|Get(acopy) (Variables|DirectionPoint|GetMoveToDirectionList) (Variables|DirectionPoint|GetCurrentDirectPoint)) (Transformation|GetActorLocation)) 1.0) (* (Variables|Movement|GetSpeed) DeltaSecond))))

(fn CanMove
  (return (and (Variables|Condition|GetIsNearPlayer) (not (Variables|Condition|GetIsNearEnemy)))))

(fn SetGoBack
  (Variables|Movement|SetStatus "NewEnumerator3")
  (return))

(fn GetBackLocation
  (params (DeltaSecond :type Float%20%28double-precision%29%20%28by%20ref%29))
  (return (* (Math|Vector|Normalize (- (CallFunction|GetBackMovetoLocation) (Transformation|GetActorLocation)) 1.0) (* (Variables|Movement|GetBackSpeed) DeltaSecond))))

(fn GetBetweenPrevCheckPointDistance
  (if (== (Variables|DirectionPoint|GetCurrentDirectPoint) 0)
    (return (Math|Vector|Distance(Vector) (Utilities|Array|Get(acopy) (Variables|DirectionPoint|GetMoveToDirectionList) (Variables|DirectionPoint|GetCurrentDirectPoint)) (Variables|DirectionPoint|GetStartPinPoint)))
    (else
      (return (Math|Vector|Distance(Vector) (Utilities|Array|Get(acopy) (Variables|DirectionPoint|GetMoveToDirectionList) (Variables|DirectionPoint|GetCurrentDirectPoint)) (Utilities|Array|Get(acopy) (Variables|DirectionPoint|GetMoveToDirectionList) (+ (Variables|DirectionPoint|GetCurrentDirectPoint) 1)))))))

(fn MovetoBack
  (params (DeltaSecond :type Float%20%28double-precision%29))
  (Transformation|SetActorLocation (+ (CallFunction|GetBackLocation DeltaSecond) (Transformation|GetActorLocation)) false false)
  (return))

(fn GetBackMovetoLocation
  (if (== (Variables|DirectionPoint|GetCurrentDirectPoint) 0)
    (return (Variables|DirectionPoint|GetStartPinPoint))
    (else
      (return (Utilities|Array|Get(acopy) (Variables|DirectionPoint|GetMoveToDirectionList) (Math|Integer|Max(Integer) (- (Variables|DirectionPoint|GetCurrentDirectPoint) 1)))))))

(fn GetTotalExpressDistance
  (for _index (range 0 (- (Utilities|Array|Length (Variables|DirectionPoint|GetDirectionList)) 1))
    (Utilities|Array|Add (Variables|Default|GetDistanceToCheckPoint) (CallFunction|GetBetweenCheckPointDistance _index))
    (LocalVariables|SetValue (+ (LocalVariables|GetValue) (CallFunction|GetBetweenCheckPointDistance _index))))
  (return (LocalVariables|GetValue)))

(fn GetBetweenCheckPointDistance
  (params (PinNumber :type Integer))
  (if (== PinNumber 0)
    (return (Math|Vector|Distance(Vector) (Variables|DirectionPoint|GetStartPinPoint) (Utilities|Array|Get(acopy) (Variables|DirectionPoint|GetMoveToDirectionList) PinNumber)))
    (else
      (return (Math|Vector|Distance(Vector) (Utilities|Array|Get(acopy) (Variables|DirectionPoint|GetMoveToDirectionList) (- PinNumber 1)) (Utilities|Array|Get(acopy) (Variables|DirectionPoint|GetMoveToDirectionList) PinNumber))))))

(fn GetCurrentDistancetoMove
  (bind _currentdirectpoint (Variables|DirectionPoint|GetCurrentDirectPoint))
  (for _index (range 0 (- _currentdirectpoint 1))
    (LocalVariables|SetLast%20Distance (+ (CallFunction|GetBetweenCheckPointDistance _index) (LocalVariables|GetLast%20Distance))))
  (return (+ (LocalVariables|GetLast%20Distance) (- (CallFunction|GetBetweenCheckPointDistance _currentdirectpoint) (Math|Vector|Distance(Vector) (Transformation|GetActorLocation) (Utilities|Array|Get(acopy) (Variables|DirectionPoint|GetMoveToDirectionList) _currentdirectpoint))))))

(fn MovePauseTimer
  (Default|SetRemainPauseTime (Variables|Default|GetHUD) (Variables|Game/Pause|GetRemainPauseTimeMs))
  (if (== (Variables|Game/Pause|GetRemainPauseTimeMs) 0)
    (bind _returnvalue (Actor|GetActorOfClass "/Game/Blueprints/Express/BP_Door.BP_Door_C"))
    (Default|OpenDoorEventEvent _returnvalue)
    (Actor|Tick|SetActorTickEnabled true)
    (Utilities|Time|ClearandInvalidateTimerbyHandle (Variables|Game/Pause|GetPauseTimerHandle))
    (bind _asbp_game_play_state (Utilities|Casting|CastToBP_GamePlayState (Game|GetGameState)))
    (Default|GameStartEventEvent _asbp_game_play_state)
    (else
      (Variables|Game/Pause|SetRemainPauseTimeMs (- (Variables|Game/Pause|GetRemainPauseTimeMs) 1))))
  (return))